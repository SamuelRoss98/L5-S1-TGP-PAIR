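; Combat game mode base that handles battle music, round resets and the end-of-battle screen.
; BeginPlay plays a fight intro, then switches to the fight track after a fixed delay, while StartNewRound delegates to ResetForNewRound.
; LoadEndOfBattleUI stops the fight track, plays victory intro and loop regardless of outcome, then shows a widget with outcome, experience earned and the names of dead enemies.
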(event EventBeginPlay
  (bind _returnvalue (Audio|SpawnSound2D "/Game/Overworld/Audio/fightintro.fightintro" 1.0 1.0 0.0 0))
  (Audio|Components|Audio|FadeIn _returnvalue 0.0 1.0 0.0 :!class /Script/Engine.AudioComponent)
  (Utilities|FlowControl|Delay 5.65)
  (bind _returnvalue_2 (Audio|SpawnSound2D "/Game/Overworld/Audio/fight.fight" 1.0 1.0 0.0 0)))

(event EventTick
  (params (DeltaSeconds :type Float%20%28single-precision%29)))

(event EventStartNewRound
  (Class|CombatGameModeBase|ResetforNewRound))

(event EventLoadEndOfBattleUI
  (params (bVictory :type Boolean) (ExpEarned :type Integer))
  (Audio|Components|Audio|Stop (stale EventBeginPlay _returnvalue_2))
  (Audio|PlaySound2D "/Game/Overworld/Audio/victoryintro.victoryintro" 1.0 1.0 0.0 0 0)
  (Utilities|FlowControl|Delay 3.8)
  (Audio|PlaySound2D "/Game/Overworld/Audio/victoryloop.victoryloop" 1.0 1.0 0.0 0 0)
  (bind _returnvalue (UserInterface|CreateWidget "/Game/Combat/UI/WBP_EndOfBattle.WBP_EndOfBattle_C"))
  (UserInterface|Viewport|AddtoViewport _returnvalue 0)
  (bind _output_get (Variables|Default|SetEndOfBattleUI _returnvalue))
  (Variables|/Game/Combat/UI/WBP_EndOfBattle.WBP_EndOfBattle_C|SetExpEarned _output_get ExpEarned)
  (if bVictory
    (Variables|/Game/Combat/UI/WBP_EndOfBattle.WBP_EndOfBattle_C|SetOutcomeText (Variables|Default|GetEndOfBattleUI) "Victory!")
    (else
      (Variables|/Game/Combat/UI/WBP_EndOfBattle.WBP_EndOfBattle_C|SetOutcomeText (Variables|Default|GetEndOfBattleUI) "Defeat!")))
  (for _array_element (Class|CombatGameModeBase|GetEnemies)
    (if (Class|CombatantPawn|IsDead _array_element)
      (bind _returnvalue_2 (UserInterface|CreateWidget "/Game/Combat/UI/WBP_DefeatedEnemyName.WBP_DefeatedEnemyName_C"))
      (Variables|/Game/Combat/UI/WBP_DefeatedEnemyName.WBP_DefeatedEnemyName_C|SetEnemyName _returnvalue_2 (.name (Class|CombatantPawn|GetBaseCharacter _array_element)))
      (Widget|Panel|AddChild (Variables|/Game/Combat/UI/WBP_EndOfBattle.WBP_EndOfBattle_C|GetEnemiesDefeatedVerticalBox (Variables|Default|GetEndOfBattleUI)) _returnvalue_2))))

(fn ConstructionScript)