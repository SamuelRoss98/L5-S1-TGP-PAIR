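; Player controller for combat that builds the HUD and handles the player's action selection menus.
; On BeginPlay it creates the combat log, action, attack, item and target list widgets, then swaps one at a time into the HUD's actions panel.
; Item and target lists are rebuilt on show from the combatant's inventory and the game mode's enemies.
; ConfirmAction writes the chosen action to the controlled combatant and signals decision completion.
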(event EventBeginPlay
  (CallFunction|CreateHUD))

(event EventTick
  (params (DeltaSeconds :type Float%20%28single-precision%29)))

(event EventPlayerDecisionStart
  (Utilities|FlowControl|Delay 0.2)
  (CallFunction|ShowActionList))

(fn ConstructionScript)

(fn CreateHUD
  ;[1 1 1] Create main HUD container.
  (bind _returnvalue (UserInterface|CreateWidget "/Game/Combat/UI/WBP_HUD.WBP_HUD_C" self))
  (bind _output_get (Variables|Default|SetHUD _returnvalue))
  (UserInterface|Viewport|AddtoViewport _output_get 0)
  ;[1 1 1] Create player action UI
  (bind _returnvalue_2 (UserInterface|CreateWidget "/Game/Combat/UI/WBP_CombatLog.WBP_CombatLog_C"))
  (Variables|Default|SetCombatLog _returnvalue_2)
  (bind _returnvalue_3 (UserInterface|CreateWidget "/Game/Combat/UI/WBP_ActionList.WBP_ActionList_C"))
  (Variables|Default|SetActionList _returnvalue_3)
  (bind _returnvalue_4 (UserInterface|CreateWidget "/Game/Combat/UI/WPB_AttackList.WPB_AttackList_C"))
  (Variables|Default|SetAttackList _returnvalue_4)
  (bind _returnvalue_5 (UserInterface|CreateWidget "/Game/Combat/UI/WBP_InventoryItemList.WBP_InventoryItemList_C"))
  (Variables|Default|SetInventoryItemList _returnvalue_5)
  (bind _returnvalue_6 (UserInterface|CreateWidget "/Game/Combat/UI/WBP_TargetList.WBP_TargetList_C"))
  (Variables|Default|SetTargetList _returnvalue_6)
  (CallFunction|ShowCombatLog))

(fn HideCurrentLeftHUD
  (Class|PanelWidget|RemoveChildat (Variables|/Game/Combat/UI/WBP_HUD.WBP_HUD_C|GetActionsPanel (Variables|Default|GetHUD))))

(fn ShowCombatLog
  (CallFunction|HideCurrentLeftHUD)
  (Widget|Panel|AddChild (Variables|/Game/Combat/UI/WBP_HUD.WBP_HUD_C|GetActionsPanel (Variables|Default|GetHUD)) (Variables|Default|GetCombatLog)))

(fn ShowActionList
  (CallFunction|HideCurrentLeftHUD)
  (Widget|Panel|AddChild (Variables|/Game/Combat/UI/WBP_HUD.WBP_HUD_C|GetActionsPanel (Variables|Default|GetHUD)) (Variables|Default|GetActionList)))

(fn ShowAttackList
  (CallFunction|HideCurrentLeftHUD)
  (Widget|Panel|AddChild (Variables|/Game/Combat/UI/WBP_HUD.WBP_HUD_C|GetActionsPanel (Variables|Default|GetHUD)) (Variables|Default|GetAttackList)))

(fn ShowRefreshedItemList
  (bind _inventoryitemlist (Variables|Default|GetInventoryItemList))
  (bind _inventoryitemsverticalbox (Variables|/Game/Combat/UI/WBP_InventoryItemList.WBP_InventoryItemList_C|GetInventoryItemsVerticalBox _inventoryitemlist))
  (Widget|Panel|ClearChildren (Variables|/Game/Combat/UI/WBP_InventoryItemList.WBP_InventoryItemList_C|GetInventoryItemsVerticalBox (Variables|Default|GetInventoryItemList)))
  ;[1 1 1] Hide previous UI and show inventory list container.
  (CallFunction|HideCurrentLeftHUD)
  (Widget|Panel|AddChild (Variables|/Game/Combat/UI/WBP_HUD.WBP_HUD_C|GetActionsPanel (Variables|Default|GetHUD)) (Variables|Default|GetInventoryItemList))
  (for _array_element (Class|InventoryComponent|GetContents (Variables|/Script/TGPPair.CombatantPawn|GetInventory (Class|CombatPlayerController|GetControlledCombatant)))
    (bind _returnvalue (UserInterface|CreateWidget "/Game/Combat/UI/WBP_InventoryItem.WBP_InventoryItem_C"))
    (Variables|/Game/Combat/UI/WBP_InventoryItem.WBP_InventoryItem_C|SetItemName _returnvalue (.name (.Item (Utilities|Struct|BreakInventorySlot _array_element))))
    (Variables|/Game/Combat/UI/WBP_InventoryItem.WBP_InventoryItem_C|SetItemQuantity _returnvalue (.Quantity (Utilities|Struct|BreakInventorySlot _array_element)))
    (Widget|Panel|AddChild _inventoryitemsverticalbox _returnvalue))
  ;[1 1 1] Create the back button
  (bind _returnvalue_2 (UserInterface|CreateWidget "/Game/Combat/UI/WBP_BackToActionsButton.WBP_BackToActionsButton_C"))
  (Widget|Panel|AddChild _inventoryitemsverticalbox _returnvalue_2))

(fn ShowRefreshedTargetList
  (bind _targetlist (Variables|Default|GetTargetList))
  (bind _targetlistverticalbox (Variables|/Game/Combat/UI/WBP_TargetList.WBP_TargetList_C|GetTargetListVerticalBox _targetlist))
  (Widget|Panel|ClearChildren (Variables|/Game/Combat/UI/WBP_TargetList.WBP_TargetList_C|GetTargetListVerticalBox (Variables|Default|GetTargetList)))
  (CallFunction|HideCurrentLeftHUD)
  (Widget|Panel|AddChild (Variables|/Game/Combat/UI/WBP_HUD.WBP_HUD_C|GetActionsPanel (Variables|Default|GetHUD)) (Variables|Default|GetTargetList))
  (bind _asbp_combat_game_mode_base (Utilities|Casting|CastToBP_CombatGameModeBase (Game|GetGameMode)))
  (for (_array_element _array_index) (Class|CombatGameModeBase|GetEnemies _asbp_combat_game_mode_base)
    (bind _returnvalue (UserInterface|CreateWidget "/Game/Combat/UI/WBP_TargetButton.WBP_TargetButton_C"))
    (Variables|/Game/Combat/UI/WBP_TargetButton.WBP_TargetButton_C|SetTargetName _returnvalue (.name (Class|CombatantPawn|GetBaseCharacter _array_element)))
    (Variables|/Game/Combat/UI/WBP_TargetButton.WBP_TargetButton_C|SetTargetIndex _returnvalue _array_index)
    (Widget|Panel|AddChild _targetlistverticalbox _returnvalue))
  (bind _returnvalue_2 (UserInterface|CreateWidget "/Game/Combat/UI/WBP_BackToActionsButton.WBP_BackToActionsButton_C"))
  (Widget|Panel|AddChild _targetlistverticalbox _returnvalue_2))

(fn ConfirmAction
  (bind _structout (Utilities|Struct|SetmembersinCombatAction (Utilities|Struct|MakeCombatAction (Variables|Default|GetCurrentActionType) (Variables|Default|GetCurrentActionData) (Variables|Default|GetCurrentActionTarget))))
  (Class|CombatantPawn|SetCurrentAction (Class|CombatPlayerController|GetControlledCombatant) _structout)
  (CallFunction|ShowCombatLog)
  (Class|CombatPlayerController|DecisionComplete))