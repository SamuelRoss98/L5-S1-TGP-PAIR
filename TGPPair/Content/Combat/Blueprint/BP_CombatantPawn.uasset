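; BP_CombatantPawn is a turn-based combat pawn that performs its chosen action when its turn comes.
; Attacks use timelines to lerp it to the target's interaction transform and back around a delayed ApplyAction, while items apply in place; every path finishes through EndAction.
; For enemies it creates a health bar widget, repositioned each tick above the resting point's projected screen position.
; DeathEvent hides the mesh.
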(event Custom|Event%20Move%20To%20Target%20For%20Attack
  ;[1 1 1] Moves this combatant to its attack target
  (bind _lerp (Timeline|MoveToTarget PlayFromStart)
    (:Update
      (Transformation|SetActorTransform (Math|Transform|Lerp(Transform) (Class|CombatantPawn|GetRestingTransform) (Class|CombatantPawn|GetInteractionTransform (Class|CombatantPawn|GetActionTargetCombatant)) _lerp)))
    (:Finished
      (CallFunction|ApplyAttackAction))))

(event Custom|Event%20Move%20To%20Rest
  ;[1 1 1] Moves the combatant back to its resting point
  (bind _newtrack_0 (Timeline|MoveToRest PlayFromStart)
    (:Update
      (Transformation|SetActorTransform (Math|Transform|Lerp(Transform) (Class|CombatantPawn|GetInteractionTransform (Class|CombatantPawn|GetActionTargetCombatant)) (Class|CombatantPawn|GetRestingTransform) _newtrack_0)))
    (:Finished
      (CallFunction|EndAction))))

(event Custom|ApplyAttackAction
  ;[1 1 1] Applies an attacking action
  (Utilities|FlowControl|Delay 0.5)
  (Class|CombatantPawn|ApplyAction)
  (Utilities|FlowControl|Delay 0.5)
  (CallFunction|EventMovetoRest))

(event Custom|ApplyItemAction
  ;[1 1 1] Applies an item action
  (Utilities|FlowControl|Delay 0.5)
  (Class|CombatantPawn|ApplyAction)
  (Utilities|FlowControl|Delay 1.0)
  (CallFunction|EndAction))

(event Collision|EventActorBeginOverlap
  (params (OtherActor :type Actor%20Object%20Reference)))

(event EventTick
  (params (DeltaSeconds :type Float%20%28single-precision%29))
  (CallFunction|PositionHUD))

(event EventTakeTurn
  (switch Utilities|FlowControl|Switch|SwitchonECombatantActionType (.actiontype (Class|CombatantPawn|GetCurrentAction))
    (:NullAction
      (CallFunction|EndAction :!label _label))
    (:Attack
      (CallFunction|EventMovetoTargetforAttack))
    (:Item
      (CallFunction|ApplyItemAction))
    (:Run
      (goto _label))))

(event EventLoadEnemyCombatantUI
  ;[1 1 1] Create HUD (this will only be called if we are an enemy combatant.
  (bind _returnvalue (UserInterface|CreateWidget "/Game/Combat/UI/WBP_EnemyHealthBars.WBP_EnemyHealthBars_C"))
  (bind _output_get (Variables|Default|SetEnemyHUD _returnvalue))
  (Variables|/Game/Combat/UI/WBP_EnemyHealthBars.WBP_EnemyHealthBars_C|SetOwningCombatant _output_get self)
  (UserInterface|Viewport|AddtoViewport _output_get 0)
  (Variables|Default|SetEnemyHUDLoaded true))

(event EventDeathEvent
  (Rendering|SetVisibility (Variables|Character|GetMesh) false false))

(fn ConstructionScript)

(fn EndAction
  (Transformation|SetActorTransform (Class|CombatantPawn|GetRestingTransform))
  (Class|CombatantPawn|EndTurn))

(fn PositionHUD
  (bind _returnvalue (Class|CombatantPawn|GetRestingTransform))
  (bind _returnvalue_2 (Game|GetPlayerController 0))
  (bind _screenlocation (Class|PlayerController|ProjectWorldLocationtoScreen _returnvalue_2 (.location _returnvalue) false))
  (if (Variables|Default|GetEnemyHUDLoaded)
    (Class|UserWidget|SetPositioninViewport (Variables|Default|GetEnemyHUD) (Math|Vector2D|MakeVector2D (.x _screenlocation) (+ (.y _screenlocation) -1e+02)) true)))