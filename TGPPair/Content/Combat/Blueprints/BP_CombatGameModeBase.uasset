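; Combat game mode base Blueprint that builds the combat UI when play begins.
; It creates the combat HUD for the first player controller, stores it and adds it to the viewport.
; It then fills the HUD's target selection box with one attack button per member of one team, each initialized with that character's index and name.
; CreateAttackButtons is an empty stub.
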(event EventBeginPlay
  (CallFunction|CreateCombatUI))

(event EventTick
  (params (DeltaSeconds :type Float%20%28single-precision%29)))

(fn ConstructionScript)

(fn CreateCombatUI
  (bind _returnvalue (UserInterface|CreateWidget "/Game/Combat/Blueprints/UI/BP_CombatHUD.BP_CombatHUD_C" (Game|GetPlayerController 0)))
  (bind _output_get (Variables|Default|SetCombatHUD _returnvalue))
  (UserInterface|Viewport|AddtoViewport _output_get 0)
  (bind _returnvalue_2 (Class|CombatGameModeBase|GetTeam false))
  (for (_array_element _array_index) _returnvalue_2
    (bind _returnvalue_3 (UserInterface|CreateWidget "/Game/Combat/Blueprints/UI/BP_AttackActionButton.BP_AttackActionButton_C"))
    (Default|InitButton _returnvalue_3 _array_index (Class|Combatant|GetCharacterName _array_element))
    (Class|VerticalBox|AddChildtoVerticalBox (Variables|/Game/Combat/Blueprints/UI/BP_CombatHUD.BP_CombatHUD_C|GetTargetSelect_VerticalBox _returnvalue) _returnvalue_3)))

(fn CreateAttackButtons)