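; Player-side combatant controller that supplies the player's action choice for combat.
; StartCombatDecisionEvent clears the completion flag and resets the decision to a null action.
; AttackDecision records an attack on a target index, prints it and marks the decision complete, ignoring further attack calls until the next reset.
; IsDecisionFinished and GetActionBP expose the completion state and chosen action, while EndDecisionProcess is an empty stub.
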(event EventBeginPlay)

(event EventTick
  (params (DeltaSeconds :type Float%20%28single-precision%29)))

(event EventStartCombatDecisionEvent
  (Variables|Default|SetDecisionComplete false)
  (Variables|Default|SetDecision (Utilities|Struct|MakeCombatantAction "NullAction" false 0)))

(fn ConstructionScript)

(fn EndDecisionProcess)

(fn IsDecisionFinished
  (return (Variables|Default|GetDecisionComplete)))

(fn AttackDecision
  (params (TargetIndex :type Integer))
  (if (not (Variables|Default|GetDecisionComplete))
    (Development|PrintString (Utilities|String|Append "Attack on target: " (Utilities|String|ToString(Integer) TargetIndex)))
    (Variables|Default|SetDecision (Utilities|Struct|MakeCombatantAction "Attack" false TargetIndex))
    (Variables|Default|SetDecisionComplete true)))

(fn GetActionBP
  (return (Variables|Default|GetDecision)))