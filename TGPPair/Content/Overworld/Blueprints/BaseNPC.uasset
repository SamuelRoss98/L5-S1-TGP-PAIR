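; BaseNPC is an overworld NPC that offers quest dialogue when the player's quest progression matches its QuestIndex.
; Tick shows or hides its TextRender on that match, and the Sphere overlap enables or disables the NPC's input.
; Pressing F while the text is visible opens a single DialogueCore widget with the quest IDs, shows the cursor and blocks look and move input.
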(event OnComponentBeginOverlap(Sphere)
  (params (OverlappedComponent :type Primitive%20Component%20Object%20Reference) (OtherActor :type Actor%20Object%20Reference) (OtherComp :type Primitive%20Component%20Object%20Reference) (OtherBodyIndex :type Integer) (bFromSweep :type Boolean) (SweepResult :type Hit%20Result%20Structure%20%28by%20ref%29))
  (Input|EnableInput (Game|GetPlayerController 0)))

(event OnComponentEndOverlap(Sphere)
  (params (OverlappedComponent :type Primitive%20Component%20Object%20Reference) (OtherActor :type Actor%20Object%20Reference) (OtherComp :type Primitive%20Component%20Object%20Reference) (OtherBodyIndex :type Integer))
  (Input|DisableInput (Game|GetPlayerController 0)))

(event EventTick
  (params (DeltaSeconds :type Float%20%28single-precision%29))
  (bind _textrender (Variables|Default|GetTextRender))
  (bind _astop_down_character (Utilities|Casting|CastToTopDownCharacter (Game|GetPlayerCharacter 0)))
  (if (== (Variables|/Game/StandardAssets/TopDownCPP/Blueprints/TopDownCharacter.TopDownCharacter_C|GetquestProgression _astop_down_character) (Variables|Default|GetquestIndex))
    (Rendering|SetVisibility _textrender true false)
    (else
      (Rendering|SetVisibility _textrender false false))))

(event Input|KeyboardEvents|F
  (params (Key :type Key%20Structure))
  (bind _returnvalue (Game|GetPlayerController 0))
  (:Pressed
    (Utilities|IsValid (Variables|Default|Getwidget)
      (:Is%20Not%20Valid
        (if (Rendering|IsVisible (Variables|Default|GetTextRender))
          (bind _returnvalue_2 (UserInterface|CreateWidget "/Game/Overworld/Widgets/Dialogue/DialogueCore.DialogueCore_C" 0 (Variables|Default|GetquestIndex) 0 (Variables|Default|GetquestProgressionIndex)))
          (Variables|/Game/Overworld/Widgets/Dialogue/DialogueCore.DialogueCore_C|SetOwner _returnvalue_2 self)
          (UserInterface|Viewport|AddtoViewport _returnvalue_2 0)
          (Variables|Default|Setwidget _returnvalue_2)
          (Variables|/Script/Engine.PlayerController|SetbShowMouseCursor _returnvalue true)
          (Input|SetIgnoreLookInput _returnvalue true)
          (Input|SetIgnoreMoveInput _returnvalue true))))))

(fn ConstructionScript)