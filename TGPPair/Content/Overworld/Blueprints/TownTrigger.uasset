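; Overworld trigger volume that marks a town as a safe zone for the TopDownCharacter.
; Entering its collision component disables the character's CanBattle flag and crossfades its music to the Ambient track.
; Leaving re-enables battles and switches the music back to Adventure1.
; Each switch fades out, waits on a one-second delay, swaps the sound, then fades in.
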(event OnComponentBeginOverlap(CollisionComponent)
  (params (OverlappedComponent :type Primitive%20Component%20Object%20Reference) (OtherActor :type Actor%20Object%20Reference) (OtherComp :type Primitive%20Component%20Object%20Reference) (OtherBodyIndex :type Integer) (bFromSweep :type Boolean) (SweepResult :type Hit%20Result%20Structure%20%28by%20ref%29))
  (bind _astop_down_character (Utilities|Casting|CastToTopDownCharacter OtherActor))
  (Variables|/Game/StandardAssets/TopDownCPP/Blueprints/TopDownCharacter.TopDownCharacter_C|SetcanBattle _astop_down_character false)
  (Audio|Components|Audio|FadeOut (Variables|/Game/StandardAssets/TopDownCPP/Blueprints/TopDownCharacter.TopDownCharacter_C|GetMusic _astop_down_character) 1.0 0.0 :!class /Script/Engine.AudioComponent)
  (Utilities|FlowControl|Delay 1.0)
  (Audio|Components|Audio|SetSound (Variables|/Game/StandardAssets/TopDownCPP/Blueprints/TopDownCharacter.TopDownCharacter_C|GetMusic _astop_down_character) "/Game/Overworld/Audio/ambient.ambient")
  (Audio|Components|Audio|FadeIn (Variables|/Game/StandardAssets/TopDownCPP/Blueprints/TopDownCharacter.TopDownCharacter_C|GetMusic _astop_down_character) 1.0 1.0 0.0 :!class /Script/Engine.AudioComponent))

(event OnComponentEndOverlap(CollisionComponent)
  (params (OverlappedComponent :type Primitive%20Component%20Object%20Reference) (OtherActor :type Actor%20Object%20Reference) (OtherComp :type Primitive%20Component%20Object%20Reference) (OtherBodyIndex :type Integer))
  (bind _astop_down_character (Utilities|Casting|CastToTopDownCharacter OtherActor))
  (Variables|/Game/StandardAssets/TopDownCPP/Blueprints/TopDownCharacter.TopDownCharacter_C|SetcanBattle _astop_down_character true)
  (Audio|Components|Audio|FadeOut (Variables|/Game/StandardAssets/TopDownCPP/Blueprints/TopDownCharacter.TopDownCharacter_C|GetMusic _astop_down_character) 1.0 0.0 :!class /Script/Engine.AudioComponent)
  (Utilities|FlowControl|Delay 1.0)
  (Audio|Components|Audio|SetSound (Variables|/Game/StandardAssets/TopDownCPP/Blueprints/TopDownCharacter.TopDownCharacter_C|GetMusic _astop_down_character) "/Game/Overworld/Audio/adventure1.adventure1")
  (Audio|Components|Audio|FadeIn (Variables|/Game/StandardAssets/TopDownCPP/Blueprints/TopDownCharacter.TopDownCharacter_C|GetMusic _astop_down_character) 1.0 1.0 0.0 :!class /Script/Engine.AudioComponent))

(fn ConstructionScript)